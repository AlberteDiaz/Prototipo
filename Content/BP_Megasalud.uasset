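; BP_Megasalud is a pickup that calls Megasalud on the first-person character that overlaps it, apparently a mega-health boost.
; Any actor overlap hides Sphere and its children before the character cast runs.
; Tick polls visibility and uses a ten-second Delay to show Sphere again.
; Both paths set Sphere1 collision to QueryAndPhysics, so the overlap handler never disables collision while Sphere is hidden.
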(event EventTick
  (params (DeltaSeconds :type Float%20%28single-precision%29))
  (bind _sphere (Variables|Default|GetSphere))
  (if (not (Rendering|IsVisible _sphere))
    (Utilities|FlowControl|Delay 1e+01)
    (Rendering|SetVisibility _sphere true true)
    (Collision|SetCollisionEnabled (Variables|Default|GetSphere1) "QueryAndPhysics")))

(event Collision|EventActorBeginOverlap
  (params (OtherActor :type Actor%20Object%20Reference))
  (Rendering|SetVisibility (Variables|Default|GetSphere) false true)
  (Collision|SetCollisionEnabled (Variables|Default|GetSphere1) "QueryAndPhysics")
  (bind _asbp_first_person_character (Utilities|Casting|CastToBP_FirstPersonCharacter OtherActor))
  (Default|Megasalud _asbp_first_person_character))

(fn ConstructionScript)